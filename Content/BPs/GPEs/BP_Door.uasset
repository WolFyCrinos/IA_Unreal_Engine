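; BP_Door is a key-locked door for the infiltration game that releases when a player holding a key reaches it.
; On BeginPlay it disables physics on the door and caches the PS_InfiltrationGame player state.
; The KeyCheck trigger filters actors by BPI_PlayerGPE, checks the player state for a key, then enables door physics and calls UseKeyMessage.
; The NextLevel trigger performs the same interface check but has no action behind it.
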(event OnComponentBeginOverlap(KeyCheck)
  (params (OverlappedComponent :type Primitive%20Component%20Object%20Reference) (OtherActor :type Actor%20Object%20Reference) (OtherComp :type Primitive%20Component%20Object%20Reference) (OtherBodyIndex :type Integer) (bFromSweep :type Boolean) (SweepResult :type Hit%20Result%20Structure%20%28by%20ref%29))
  (if (Utilities|DoesObjectImplementInterface OtherActor "/Game/BPs/Interfaces/BPI_PlayerGPE.BPI_PlayerGPE_C")
    (bind _haskey (Default|GetCurrentKey (Variables|Default|GetPlayerState)))
    (if _haskey
      (Physics|SetSimulatePhysics (Variables|Default|GetDoor) true)
      (Class|BPIPlayerGPE|UseKey(Message) (Variables|Default|GetPlayerState)))))

(event OnComponentBeginOverlap(NextLevel)
  (params (OverlappedComponent :type Primitive%20Component%20Object%20Reference) (OtherActor :type Actor%20Object%20Reference) (OtherComp :type Primitive%20Component%20Object%20Reference) (OtherBodyIndex :type Integer) (bFromSweep :type Boolean) (SweepResult :type Hit%20Result%20Structure%20%28by%20ref%29))
  (if (Utilities|DoesObjectImplementInterface OtherActor "/Game/BPs/Interfaces/BPI_PlayerGPE.BPI_PlayerGPE_C")
    _))

(event EventBeginPlay
  (Physics|SetSimulatePhysics (Variables|Default|GetDoor) false)
  (bind _asps_infiltration_game (Utilities|Casting|CastToPS_InfiltrationGame (Game|GetPlayerState 0)))
  (Variables|Default|SetPlayerState _asps_infiltration_game))

(fn ConstructionScript)