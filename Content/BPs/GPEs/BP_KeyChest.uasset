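; Coin-gated key chest that opens when the player can pay its coin cost.
; On a trigger overlap by an actor implementing BPI_PlayerGPE, it compares the coin count from the cached PS_InfiltrationGame player state against CoinNeededForKey.
; If affordable, it notifies the player state of the opening and coin spend, then enables physics on the Door so it swings or falls free.
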(event OnComponentBeginOverlap(Trigger)
  (params (OverlappedComponent :type Primitive%20Component%20Object%20Reference) (OtherActor :type Actor%20Object%20Reference) (OtherComp :type Primitive%20Component%20Object%20Reference) (OtherBodyIndex :type Integer) (bFromSweep :type Boolean) (SweepResult :type Hit%20Result%20Structure%20%28by%20ref%29))
  (bind _playerstate (Variables|Default|GetPlayerState))
  (if (Utilities|DoesObjectImplementInterface OtherActor "/Game/BPs/Interfaces/BPI_PlayerGPE.BPI_PlayerGPE_C")
    (bind _coinvalue (Default|GetCurrentCoin _playerstate))
    (bind _returnvalue (CallFunction|CheckCoinforKey _coinvalue))
    (if _returnvalue
      (Class|BPIPlayerGPE|OpenChest(Message) _playerstate)
      (Class|BPIPlayerGPE|UseCoin(Message) _playerstate (Variables|Default|GetCoinNeededForKey))
      (Physics|SetSimulatePhysics (Variables|Default|GetDoor) true))))

(event Custom|TestKeyChest
  (bind _playerstate (Variables|Default|GetPlayerState))
  (bind _coinvalue (Default|GetCurrentCoin _playerstate))
  (bind _returnvalue (CallFunction|CheckCoinforKey _coinvalue))
  (if _returnvalue
    (Class|BPIPlayerGPE|OpenChest(Message) _playerstate)
    (Class|BPIPlayerGPE|UseCoin(Message) _playerstate (Variables|Default|GetCoinNeededForKey))
    (Physics|SetSimulatePhysics (Variables|Default|GetDoor) true)))

(event EventBeginPlay
  (Physics|SetSimulatePhysics (Variables|Default|GetDoor) false)
  (bind _asps_infiltration_game (Utilities|Casting|CastToPS_InfiltrationGame (Game|GetPlayerState 0)))
  (Variables|Default|SetPlayerState _asps_infiltration_game))

(fn ConstructionScript)

(fn CheckCoinforKey
  (params (CurrentCoins :type Integer))
  (return (>= CurrentCoins (Variables|Default|GetCoinNeededForKey))))