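; Game mode for the infiltration game that creates the player widget and manages level-based respawns, lives and game over.
; On BeginPlay it loads the current level from the "hgs" save slot and respawns the player at the matching "Level"+number PlayerStart.
; Deaths respawn the player and update PlayerState lives.
; At zero, lives reset and, given an existing save, a beaten coin high score saves with the level before MainMenu opens.
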(event Custom|NextLevel
  (bind _result (Math|Integer|IncrementInt (Variables|Default|GetCurrentLevel))
    (:%20%20
      (Development|PrintString (Utilities|String|Append "NextLevel: " (Utilities|String|ToString(Integer) _result))))))

(event Custom|RestartGameLevel
  (params (Controller :type Controller%20Object%20Reference))
  (bind _output_get (Variables|Default|SetController Controller))
  (Actor|DestroyActor (Pawn|GetControlledPawn _output_get))
  (Class|GameModeBase|RestartPlayeratPlayerStart (Variables|Default|GetController) (Class|GameModeBase|FindPlayerStart (Variables|Default|GetController) (Utilities|String|Append "Level" (Utilities|String|ToString(Integer) (Variables|Default|GetCurrentLevel))))))

(event Custom|Killed
  (params (Controller :type Controller%20Object%20Reference))
  (Default|CallGAMEOVER)
  (CallFunction|RestartGameLevel Controller)
  (CallFunction|IsGameOver))

(event Custom|IsGameOver
  (Default|Killed (stale EventBeginPlay _output_get_2))
  (bind _life (Default|GetCurrentLife (stale EventBeginPlay _output_get_2)))
  (bind _returnvalue (CallFunction|CheckPlayerLife _life))
  (if _returnvalue
    (Default|ResetLife (stale EventBeginPlay _output_get_2))
    (bind _returnvalue_2 (SaveGame|DoesSaveGameExist "hgs"))
    (if _returnvalue_2
      (bind _returnvalue_3 (SaveGame|LoadGamefromSlot "hgs"))
      (bind _asbp_save (Utilities|Casting|CastToBP_Save _returnvalue_3))
      (bind _coinvalue (Default|GetCurrentCoin (stale EventBeginPlay _output_get_2)))
      (if (< (Variables|/Game/BPs/Game/BP_Save.BP_Save_C|GetHighScore _asbp_save) _coinvalue)
        (bind _returnvalue_4 (SaveGame|CreateSaveGameObject "/Game/BPs/Game/BP_Save.BP_Save_C"))
        (Variables|/Game/BPs/Game/BP_Save.BP_Save_C|SetCurrentLevel _returnvalue_4 (Variables|Default|GetCurrentLevel))
        (Variables|/Game/BPs/Game/BP_Save.BP_Save_C|SetHighScore _returnvalue_4 _coinvalue)
        (SaveGame|SaveGametoSlot _returnvalue_4 "hgs"))
      (Game|OpenLevel(byObjectReference) "/Game/ThirdPerson/Maps/MainMenu.MainMenu")
      (else
        (Development|PrintString "NO save found" true true "(R=1.000000,G=0.000000,B=0.000000,A=1.000000)")))))

(event EventBeginPlay
  (bind _returnvalue (Game|GetPlayerController 0))
  (Utilities|FlowControl|Sequence
    (:then_0
      (bind _returnvalue_2 (UserInterface|CreateWidget "/Game/BPs/Widgets/WBP_InfiltrationGame.WBP_InfiltrationGame_C" _returnvalue))
      (bind _output_get (Variables|Default|SetPlayerWidget _returnvalue_2))
      (UserInterface|Viewport|AddtoPlayerScreen _output_get)
      (bind _asps_infiltration_game (Utilities|Casting|CastToPS_InfiltrationGame (Variables|/Script/Engine.Controller|GetPlayerState _returnvalue)))
      (bind _output_get_2 (Variables|Default|SetAs%20PS%20Infiltration%20Game _asps_infiltration_game))
      (bind _returnvalue_3 (SaveGame|DoesSaveGameExist "hgs"))
      (if _returnvalue_3
        (bind _returnvalue_4 (SaveGame|LoadGamefromSlot "hgs"))
        (bind _asbp_save (Utilities|Casting|CastToBP_Save _returnvalue_4))
        (bind _output_get_3 (Variables|Default|SetCurrentLevel (Variables|/Game/BPs/Game/BP_Save.BP_Save_C|GetCurrentLevel _asbp_save)))
        (Development|PrintString (Utilities|String|Append "Level: " (Utilities|String|ToString(Integer) _output_get_3)))
        (Utilities|FlowControl|Delay 0.2)
        (CallFunction|RestartGameLevel _returnvalue)))))

(fn ConstructionScript)

(fn CheckPlayerLife
  (params (CurrentLife :type Integer))
  (return (<= CurrentLife 0)))